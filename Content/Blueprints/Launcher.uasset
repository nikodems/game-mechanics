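; Launcher Blueprint that fires projectiles on a Z key press, configured through checkboxes in a sample UI widget.
; On each press it reads the checkboxes to choose single or multiple shots and set the ricochet, pierce and split flags.
; It then calls FireProjectile, whose logic is not defined in this graph.
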(event Input|KeyboardEvents|Z
  (params (Key :type Key%20Structure))
  (:Pressed
    (if (Class|CheckBox|IsChecked (Variables|/Game/Blueprints/SampleUI.SampleUI_C|GetMultipleProj (Variables|/Game/Blueprints/Widget.Widget_C|GetSampleUI (Variables|Default|Getwidget))))
      (Variables|Default|SetnumOfProjToFire 5)
      (else
        (Variables|Default|SetnumOfProjToFire 1)))
    (Variables|Default|SetprojectileRicochet (Class|CheckBox|IsChecked (Variables|/Game/Blueprints/SampleUI.SampleUI_C|GetBounce (Variables|/Game/Blueprints/Widget.Widget_C|GetSampleUI (Variables|Default|Getwidget)))))
    (Variables|Default|SetprojectilePierce (Class|CheckBox|IsChecked (Variables|/Game/Blueprints/SampleUI.SampleUI_C|GetPierce (Variables|/Game/Blueprints/Widget.Widget_C|GetSampleUI (Variables|Default|Getwidget)))))
    (Variables|Default|SetprojectileSplit (Class|CheckBox|IsChecked (Variables|/Game/Blueprints/SampleUI.SampleUI_C|GetSplit (Variables|/Game/Blueprints/Widget.Widget_C|GetSampleUI (Variables|Default|Getwidget)))))
    (Class|MyActor|FireProjectile)))

(fn ConstructionScript)