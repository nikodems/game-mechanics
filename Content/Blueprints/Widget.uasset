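; Actor Blueprint that toggles an on-screen SampleUI widget with the Enter key.
; BeginPlay creates the widget once and stores it, and a WidgetAlive flag tracks whether it is showing.
; Each press either adds it to the viewport with Game and UI input focused on it and the cursor visible, or removes it, hides the cursor and restores game-only input.
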(event EventBeginPlay
  ;[1 1 1] Create widget and assign it to SampleUI
  (bind _returnvalue (UserInterface|CreateWidget "/Game/Blueprints/SampleUI.SampleUI_C"))
  (Variables|Default|SetSampleUI _returnvalue))

(event Input|KeyboardEvents|Enter
  (params (Key :type Key%20Structure))
  (bind _returnvalue (Game|GetPlayerController 0))
  (bind _sampleui (Variables|Default|GetSampleUI))
  (:Pressed
    (if (Variables|Default|GetwidgetAlive)
      ;[1 1 1] If widget is showing
      (Widget|RemovefromParent (Variables|Default|GetSampleUI)) ; Remove widget
      (Variables|/Script/Engine.PlayerController|SetbShowMouseCursor _returnvalue false) ; hide cursor
      (Input|SetInputModeGameOnly _returnvalue) ; allow input to game
      (Variables|Default|SetwidgetAlive false)
      (else
        ;[1 1 1] If widget is not showing
        (UserInterface|Viewport|AddtoViewport _sampleui 0) ; render widget
        (Input|SetInputModeGameandUI (Game|GetPlayerController 0) _sampleui "DoNotLock" true) ; allow input to ui
        (Variables|/Script/Engine.PlayerController|SetbShowMouseCursor (Game|GetPlayerController 0) true) ; show mouse cursor
        (Variables|Default|SetwidgetAlive true)))))

(fn ConstructionScript)